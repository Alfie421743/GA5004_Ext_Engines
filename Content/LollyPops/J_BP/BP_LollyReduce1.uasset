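; BP_LollyReduce1 is an interactable lolly that shrinks with each interaction and awards the player a point when used up.
; Overlapping its collision box sets the player character's interact flag and registers the lolly as the current interaction.
; Each CE_Reduce call lowers a click counter and mesh scale; at one, it restores both, prints a message and increments the player's score.
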(event `self.ReceiveBeginPlay`
  ;[1 1 1] Comment
  (bind _asbp_third_person_character (cast `/Game/LollyPops/ThirdPerson/Blueprints/BP_ThirdPersonCharacter` (`GameplayStatics.GetPlayerCharacter` 0)))
  (set `self.As BP Third Person Character` _asbp_third_person_character))

(event `CE_Reduce`
  ;[1 1 1] Comment
  (if (!= (`self.Var_ClickCount`) 1)
    (set `self.ReduceLolly` (+ (`self.ReduceLolly`) (-0.1 -0.1 -0.1)))
    (`/Engine/EditorBlueprintResources/StandardMacros.DecrementInt` (`self.Var_ClickCount`)
      (:`  `
        (`SceneComponent.SetRelativeScale3D` (`self.SM_Lolly`) (`self.ReduceLolly`))))
    (else
      ;[1 1 1] reset
      (bind _output_get (set `self.ReduceLolly` (1.0 1.0 1.0)))
      (`SceneComponent.SetRelativeScale3D` (`self.SM_Lolly`) _output_get)
      (set `self.Var_ClickCount` 10)
      (`KismetSystemLibrary.PrintString` "1st Lolly" true true (struct :`G` 0.66 :`B` 1.0 :`A` 1.0) 10.0)
      (bind _asbp_third_person_character (cast `/Game/LollyPops/ThirdPerson/Blueprints/BP_ThirdPersonCharacter` (`GameplayStatics.GetPlayerCharacter` 0)))
      (set `/Game/LollyPops/ThirdPerson/Blueprints/BP_ThirdPersonCharacter.Var_Score` (+ (`/Game/LollyPops/ThirdPerson/Blueprints/BP_ThirdPersonCharacter.Var_Score` _asbp_third_person_character) 1) _asbp_third_person_character))))

(event `self.C+Box.OnComponentBeginOverlap`
  (params (OverlappedComponent :type "PrimitiveComponent Object Reference") (OtherActor :type "Actor Object Reference") (OtherComp :type "PrimitiveComponent Object Reference") (OtherBodyIndex :type Integer) (bFromSweep :type Boolean) (SweepResult :type "HitResult Structure (by ref)"))
  (bind _as_bp_third_person_character (`self.As BP Third Person Character`))
  ;[1 1 1] is this the active player
  (if (== OtherActor (`GameplayStatics.GetPlayerCharacter` 0))
    (set `/Game/LollyPops/ThirdPerson/Blueprints/BP_ThirdPersonCharacter.Var_Interact` true _as_bp_third_person_character)
    (set `/Game/LollyPops/ThirdPerson/Blueprints/BP_ThirdPersonCharacter.currentInteraction` self _as_bp_third_person_character)))

(fn `UserConstructionScript`)
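; Lollipop actor that the third-person character can lick while inside its box area, playing a sound and animating the candy's size.
; Overlap opens and closes a gate on the IA_Lick input.
; Each lick restarts a timeline lerping mesh scale between the BeginPlay scale and a slightly larger one, despite the "Reduce" naming.
; An E key handler adjusts a vector nothing here reads; a second timeline chain never runs.
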(event `self.ReceiveBeginPlay`
  (bind (_returnvalue_location _returnvalue_rotation _returnvalue_scale) (`KismetMathLibrary.BreakTransform` (`SceneComponent.GetRelativeTransform` (`self.SM_Lolly`))))
  (set `self.Var_ReduceSize` (`KismetMathLibrary.MakeTransform` _returnvalue_location _returnvalue_rotation _returnvalue_scale))
  (set `self.Var_IncreaseSize` (`KismetMathLibrary.MakeTransform` (0.0 0.0 0.0) (struct) (- _returnvalue_scale (-0.1 -0.1 -0.1))))
  (`self.EnableInput` (`GameplayStatics.GetPlayerController` 0)))

(event `EnhancedInput|/Game/LollyPops/J_Input/IA_Lick`
  (params (ActionValue :type Boolean) (ElapsedSeconds :type "Float (double-precision)") (TriggeredSeconds :type "Float (double-precision)") (InputAction :type "InputAction Object Reference" :default "/Game/LollyPops/J_Input/IA_Lick.IA_Lick"))
  (:`Started`
    (`/Engine/EditorBlueprintResources/StandardMacros.Gate` true :!label _label
      (:`Exit`
        (`GameplayStatics.PlaySoundAtLocation` "/Game/LollyPops/J_Audio/FS_Gravel_02.FS_Gravel_02" (`self.K2_GetActorLocation`) (struct) 1.0 1.0 0.0 null null null null)
        (bind (_direction _ft_reducelollysize) (`Timeline|TL_ReduceLollySize` :!via `PlayFromStart`)
          (:`Update`
            (bind (_returnvalue_location _returnvalue_rotation _returnvalue_scale) (`KismetMathLibrary.BreakTransform` (`KismetMathLibrary.TLerp` (`self.Var_ReduceSize`) (`self.Var_IncreaseSize`) _ft_reducelollysize)))
            (`SceneComponent.SetRelativeScale3D` (`self.SM_Lolly`) _returnvalue_scale)))))))

(event `self.BC_LollyArea.OnComponentBeginOverlap`
  (params (OverlappedComponent :type "PrimitiveComponent Object Reference") (OtherActor :type "Actor Object Reference") (OtherComp :type "PrimitiveComponent Object Reference") (OtherBodyIndex :type Integer) (bFromSweep :type Boolean) (SweepResult :type "HitResult Structure (by ref)"))
  (cast `/Game/LollyPops/ThirdPerson/Blueprints/BP_ThirdPersonCharacter` OtherActor)
  (goto _label :!via `Open`))

(event `self.BC_LollyArea.OnComponentEndOverlap`
  (params (OverlappedComponent :type "PrimitiveComponent Object Reference") (OtherActor :type "Actor Object Reference") (OtherComp :type "PrimitiveComponent Object Reference") (OtherBodyIndex :type Integer))
  (cast `/Game/LollyPops/ThirdPerson/Blueprints/BP_ThirdPersonCharacter` OtherActor)
  (goto _label :!via `Close`))

(event `Key|E`
  (params (Key :type "Key Structure"))
  (:`Pressed`
    (set `self.Var_ReduceVector` (+ (`self.Var_ReduceVector`) (-0.1 -0.1 -0.1)))))

(fn `UserConstructionScript`)
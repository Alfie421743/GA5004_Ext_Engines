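; BC_BP_BuyBeetroot is a trigger actor that shows a billboard when the player character enters its box; it holds no purchase logic.
; BeginPlay caches the player's BC_BP_ThirdPersonCharacter, and begin overlap shows the billboard only for that character.
; End overlap compares the overlapped component, not the other actor, to the character, so any actor leaving the box hides the billboard.
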(event `self.ReceiveBeginPlay`
  (bind _asbc_bp_third_person_character (cast `/Game/CropCrazy/ThirdPerson/Blueprints/BC_BP_ThirdPersonCharacter` (`GameplayStatics.GetPlayerCharacter` 0)))
  (set `self.REF_Character` _asbc_bp_third_person_character))

(event `self.Box.OnComponentBeginOverlap`
  (params (OverlappedComponent :type "PrimitiveComponent Object Reference") (OtherActor :type "Actor Object Reference") (OtherComp :type "PrimitiveComponent Object Reference") (OtherBodyIndex :type Integer) (bFromSweep :type Boolean) (SweepResult :type "HitResult Structure (by ref)"))
  (if (== OtherActor (`self.REF_Character`))
    (`SceneComponent.SetVisibility` (`self.Billboard`) true false)))

(event `self.Box.OnComponentEndOverlap`
  (params (OverlappedComponent :type "PrimitiveComponent Object Reference") (OtherActor :type "Actor Object Reference") (OtherComp :type "PrimitiveComponent Object Reference") (OtherBodyIndex :type Integer))
  (if (not (== OverlappedComponent (`self.REF_Character`)))
    (`SceneComponent.SetVisibility` (`self.Billboard`) false false)))

(fn `UserConstructionScript`)
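; BC_BP_MushroomHarvested is a harvested mushroom pickup that the player collects by running over it.
; On BeginPlay it casts player 0's character to BC_BP_ThirdPersonCharacter and caches the reference.
; When the Mushroom_Collision component begins overlapping that character, it increments the character's MushroomAmount and destroys itself.
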(event `self.ReceiveBeginPlay`
  ;[0 1 0] Reference the player
  (bind _asbc_bp_third_person_character (cast `/Game/CropCrazy/ThirdPerson/Blueprints/BC_BP_ThirdPersonCharacter` (`GameplayStatics.GetPlayerCharacter` 0)))
  (set `self.REF_Character` _asbc_bp_third_person_character))

(event `self.Mushroom_Collision.OnComponentBeginOverlap`
  (params (OverlappedComponent :type "PrimitiveComponent Object Reference") (OtherActor :type "Actor Object Reference") (OtherComp :type "PrimitiveComponent Object Reference") (OtherBodyIndex :type Integer) (bFromSweep :type Boolean) (SweepResult :type "HitResult Structure (by ref)"))
  (bind _ref_character (`self.REF_Character`))
  ;[0 1 0] When the Player Runs Over the Mushroom, Add 1 to Player 1 and Destroy the Mushroom
  (if (== OtherActor _ref_character)
    (bind _result (`/Engine/EditorBlueprintResources/StandardMacros.IncrementInt` (`/Game/CropCrazy/ThirdPerson/Blueprints/BC_BP_ThirdPersonCharacter.MushroomAmount` _ref_character))
      (:`  `
        (set `/Game/CropCrazy/ThirdPerson/Blueprints/BC_BP_ThirdPersonCharacter.MushroomAmount` _result _ref_character)
        (`self.K2_DestroyActor`)))))

(fn `UserConstructionScript`)
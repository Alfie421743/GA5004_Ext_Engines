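; BP_BeetrootHarvested is a harvested beetroot pickup that the player collects by running over it.
; On BeginPlay it casts player 0's character to BP_ThirdPersonCharacter and caches the reference.
; When its collision component overlaps that player, it increments the character's P1AmountOfBeetroot count and destroys itself.
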(event `self.ReceiveBeginPlay`
  ;[0.003 1 0] Character Reference
  (bind _asbp_third_person_character (cast `/Game/CropCrazy/ThirdPerson/Blueprints/BP_ThirdPersonCharacter` (`GameplayStatics.GetPlayerCharacter` 0)))
  (set `self.REF_Character` _asbp_third_person_character))

(event `self.Beetroot_Collision.OnComponentBeginOverlap`
  (params (OverlappedComponent :type "PrimitiveComponent Object Reference") (OtherActor :type "Actor Object Reference") (OtherComp :type "PrimitiveComponent Object Reference") (OtherBodyIndex :type Integer) (bFromSweep :type Boolean) (SweepResult :type "HitResult Structure (by ref)"))
  (bind _ref_character (`self.REF_Character`))
  ;[0 1 0] When the Player Runs Over the Beetroot, Add 1 to the Player and Destroy the Beetroot
  (if (== OtherActor (`GameplayStatics.GetPlayerCharacter` 0))
    (bind _result (`/Engine/EditorBlueprintResources/StandardMacros.IncrementInt` (`/Game/CropCrazy/ThirdPerson/Blueprints/BP_ThirdPersonCharacter.P1_AmountOfBeetroot` _ref_character))
      (:`  `
        (set `/Game/CropCrazy/ThirdPerson/Blueprints/BP_ThirdPersonCharacter.P1_AmountOfBeetroot` _result _ref_character)
        (`self.K2_DestroyActor`)))))

(fn `UserConstructionScript`)
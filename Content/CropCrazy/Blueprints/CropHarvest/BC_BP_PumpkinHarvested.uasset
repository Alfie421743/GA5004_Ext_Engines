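; Harvested pumpkin pickup that either of two players collects by running over it.
; On BeginPlay it caches both BC_BP_ThirdPersonCharacter players by their index in GetAllActorsOfClass.
; When Pumpkin_Collision begins overlapping one of them, it increments that player's PumpkinAmount and destroys itself.
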(event `self.ReceiveBeginPlay`
  ;[0 1 0] Reference the character
  (bind _outactors (`GameplayStatics.GetAllActorsOfClass` "/Game/CropCrazy/ThirdPerson/Blueprints/BC_BP_ThirdPersonCharacter.BC_BP_ThirdPersonCharacter_C"))
  (set `self.REF_Player1` (`|GetArrayItem` _outactors))
  (set `self.REF_Player2` (`|GetArrayItem` _outactors 1)))

(event `self.Pumpkin_Collision.OnComponentBeginOverlap`
  (params (OverlappedComponent :type "PrimitiveComponent Object Reference") (OtherActor :type "Actor Object Reference") (OtherComp :type "PrimitiveComponent Object Reference") (OtherBodyIndex :type Integer) (bFromSweep :type Boolean) (SweepResult :type "HitResult Structure (by ref)"))
  (bind _ref_player1 (`self.REF_Player1`))
  (bind _ref_player2 (`self.REF_Player2`))
  ;[0 1 0] When the Player Runs Over the Pumpkin, Add 1 to the Player and Destroy the Pumpkin
  (if (== OtherActor _ref_player1)
    (bind _result (`/Engine/EditorBlueprintResources/StandardMacros.IncrementInt` (`/Game/CropCrazy/ThirdPerson/Blueprints/BC_BP_ThirdPersonCharacter.PumpkinAmount` _ref_player1))
      (:`  `
        (set `/Game/CropCrazy/ThirdPerson/Blueprints/BC_BP_ThirdPersonCharacter.PumpkinAmount` _result _ref_player1)
        (`self.K2_DestroyActor` :!label _label)))
    (elif (== OtherActor _ref_player2)
      (bind _result_2 (`/Engine/EditorBlueprintResources/StandardMacros.IncrementInt` (`/Game/CropCrazy/ThirdPerson/Blueprints/BC_BP_ThirdPersonCharacter.PumpkinAmount` _ref_player2))
        (:`  `
          (set `/Game/CropCrazy/ThirdPerson/Blueprints/BC_BP_ThirdPersonCharacter.PumpkinAmount` _result_2 _ref_player2)
          (goto _label))))))

(fn `UserConstructionScript`)
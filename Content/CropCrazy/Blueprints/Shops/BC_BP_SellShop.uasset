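; Sell shop actor for two local players that opens a selling menu when something enters its Box trigger.
; Player 0's character gets the P1 widget, while any other actor opens the P2 widget on controller 1.
; Each widget switches input to Game and UI and focuses its beet amount button for controller support.
; End overlap removes both widgets, but restores game-only input and hides the cursor only for controller 0.
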(event `self.ReceiveBeginPlay`
  ;[0 1 0] Set Text "Sell Shop"
  (set `Text3DComponent.Text` "Sell" (`self.TXT_SellShop`))
  ;[0 1 0] Cast to Player
  (bind _asbc_bp_third_person_character (cast `/Game/CropCrazy/ThirdPerson/Blueprints/BC_BP_ThirdPersonCharacter` (`GameplayStatics.GetPlayerCharacter` 0)))
  (set `self.REF_Character` _asbc_bp_third_person_character))

(event `self.Box.OnComponentBeginOverlap`
  (params (OverlappedComponent :type "PrimitiveComponent Object Reference") (OtherActor :type "Actor Object Reference") (OtherComp :type "PrimitiveComponent Object Reference") (OtherBodyIndex :type Integer) (bFromSweep :type Boolean) (SweepResult :type "HitResult Structure (by ref)"))
  (bind _returnvalue (`GameplayStatics.GetPlayerController` 1))
  (bind _returnvalue_2 (`GameplayStatics.GetPlayerController` 0))
  ;[0 1 0] When the Player is Close to The Shop Open the "Sell Shop" Widget
  (if (== OtherActor (`self.REF_Character`))
    (bind _returnvalue_3 (`|GenericCreateObject` _returnvalue_2 "/Game/CropCrazy/UI/BC_WBP_P1SellShop.BC_WBP_P1SellShop_C"))
    (`UserWidget.AddToViewport` _returnvalue_3 0)
    (`WidgetBlueprintLibrary.SetInputMode_GameAndUIEx` _returnvalue_2 null)
    (set `PlayerController.bShowMouseCursor` true _returnvalue)
    ;[0 1 0] Add Controller Support To Sell Shop
    (`Widget.SetKeyboardFocus` (`/Game/CropCrazy/UI/BC_WBP_P1SellShop.BT_BeetAmount` _returnvalue_3))
    (else
      (bind _returnvalue_4 (`|GenericCreateObject` _returnvalue "/Game/CropCrazy/UI/BC_WBP_P2SellShop.BC_WBP_P2SellShop_C"))
      (`UserWidget.AddToViewport` _returnvalue_4 0)
      (`WidgetBlueprintLibrary.SetInputMode_GameAndUIEx` _returnvalue null)
      ;[0 1 0] Add Controller Support To Sell Shop
      (`Widget.SetKeyboardFocus` (`/Game/CropCrazy/UI/BC_WBP_P2SellShop.BT_BeetAmount` _returnvalue_4)))))

(event `self.Box.OnComponentEndOverlap`
  (params (OverlappedComponent :type "PrimitiveComponent Object Reference") (OtherActor :type "Actor Object Reference") (OtherComp :type "PrimitiveComponent Object Reference") (OtherBodyIndex :type Integer))
  (bind _returnvalue (`GameplayStatics.GetPlayerController` 0))
  ;[0 1 0] When the Player Moves Away From the Shop, Close the "Sell Shop" Widget
  (if (not (== OverlappedComponent (`GameplayStatics.GetPlayerCharacter` 0)))
    (`Widget.RemoveFromParent` (stale `self.Box.OnComponentBeginOverlap` _returnvalue_3))
    (`Widget.RemoveFromParent` (stale `self.Box.OnComponentBeginOverlap` _returnvalue_4))
    (`WidgetBlueprintLibrary.SetInputMode_GameOnly` _returnvalue)
    (set `PlayerController.bShowMouseCursor` false _returnvalue)))

(fn `UserConstructionScript`)
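; BP_SellShop is a shop actor that opens the WBP_SellShop selling menu when the player enters its box trigger.
; Entering clears existing widgets, shows the menu with cursor and Game and UI input, ignores look input, and focuses the beet button for controller support.
; End overlap compares the overlapped component, not the other actor, to the player, and removes the menu and restores game-only input without re-enabling look input.
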(event `self.ReceiveBeginPlay`
  ;[0 1 0] Set Text "Sell Shop"
  (set `Text3DComponent.Text` "Sell" (`self.TXT_SellShop`))
  ;[0 1 0] Cast to Player
  (bind _asbp_third_person_character (cast `/Game/CropCrazy/ThirdPerson/Blueprints/BP_ThirdPersonCharacter` (`GameplayStatics.GetPlayerCharacter` 0)))
  (set `self.REF_Character` _asbp_third_person_character))

(event `self.Box.OnComponentBeginOverlap`
  (params (OverlappedComponent :type "PrimitiveComponent Object Reference") (OtherActor :type "Actor Object Reference") (OtherComp :type "PrimitiveComponent Object Reference") (OtherBodyIndex :type Integer) (bFromSweep :type Boolean) (SweepResult :type "HitResult Structure (by ref)"))
  (bind _returnvalue (`GameplayStatics.GetPlayerController` 0))
  ;[0 1 0] When the Player is Close to The Shop Open the "Sell Shop" Widget
  (if (== OtherActor (`GameplayStatics.GetPlayerCharacter` 0))
    (`WidgetLayoutLibrary.RemoveAllWidgets`)
    (bind _returnvalue_2 (`|GenericCreateObject` "/Game/CropCrazy/UI/WBP_SellShop.WBP_SellShop_C"))
    (`UserWidget.AddToViewport` _returnvalue_2 0)
    (`WidgetBlueprintLibrary.SetInputMode_GameAndUIEx` _returnvalue null)
    (set `PlayerController.bShowMouseCursor` true _returnvalue)
    (`Controller.SetIgnoreLookInput` _returnvalue true)
    ;[0 1 0] Add Controller Support To Sell Shop
    (`Widget.SetKeyboardFocus` (`/Game/CropCrazy/UI/WBP_SellShop.BT_BeetAmount` _returnvalue_2))))

(event `self.Box.OnComponentEndOverlap`
  (params (OverlappedComponent :type "PrimitiveComponent Object Reference") (OtherActor :type "Actor Object Reference") (OtherComp :type "PrimitiveComponent Object Reference") (OtherBodyIndex :type Integer))
  (bind _returnvalue (`GameplayStatics.GetPlayerController` 0))
  ;[0 1 0] When the Player Moves Away From the Shop, Close the "Sell Shop" Widget
  (if (not (== OverlappedComponent (`GameplayStatics.GetPlayerCharacter` 0)))
    (`Widget.RemoveFromParent` (stale `self.Box.OnComponentBeginOverlap` _returnvalue_2))
    (`WidgetBlueprintLibrary.SetInputMode_GameOnly` _returnvalue)
    (set `PlayerController.bShowMouseCursor` false _returnvalue)))

(fn `UserConstructionScript`)
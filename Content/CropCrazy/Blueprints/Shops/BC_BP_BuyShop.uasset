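; Shop actor for local two-player play that labels itself "Buy" and opens a purchase menu when a player walks into its Interact volume.
; Player 0's character gets the P1 widget and mouse cursor; any other actor triggers the P2 widget, both with controller focus and look input ignored.
; End overlap compares the component to a controller, removes both widgets, restores only player 0's input mode and cursor, and adds a new HUD without re-enabling look.
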(event `self.ReceiveBeginPlay`
  ;[0 1 0] Set Text "Buy Shop"
  (set `Text3DComponent.Text` "Buy" (`self.TXT_Buy`))
  ;[0 1 0] Cast to Player
  (bind _asbc_bp_third_person_character (cast `/Game/CropCrazy/ThirdPerson/Blueprints/BC_BP_ThirdPersonCharacter` (`GameplayStatics.GetPlayerCharacter` 0)))
  (set `self.REF_Character` _asbc_bp_third_person_character))

(event `self.Interact.OnComponentBeginOverlap`
  (params (OverlappedComponent :type "PrimitiveComponent Object Reference") (OtherActor :type "Actor Object Reference") (OtherComp :type "PrimitiveComponent Object Reference") (OtherBodyIndex :type Integer) (bFromSweep :type Boolean) (SweepResult :type "HitResult Structure (by ref)"))
  (bind _returnvalue (`GameplayStatics.GetPlayerController` 1))
  (bind _returnvalue_2 (`GameplayStatics.GetPlayerController` 0))
  ;[0 1 0] When Player 1 is Close to The Shop Open the "Buy Shop" Widget
  (if (== OtherActor (`self.REF_Character`))
    (bind _returnvalue_3 (`|CreateWidget` "/Game/CropCrazy/UI/BC_WBP_P1BuyShop.BC_WBP_P1BuyShop_C" _returnvalue_2))
    (`UserWidget.AddToViewport` _returnvalue_3 0)
    (`WidgetBlueprintLibrary.SetInputMode_GameAndUIEx` _returnvalue_2 null)
    (set `PlayerController.bShowMouseCursor` true _returnvalue_2)
    (`Controller.SetIgnoreLookInput` _returnvalue_2 true)
    ;[0 1 0] Add Controller Support to Player 1Buy Shop
    (`Widget.SetKeyboardFocus` (`/Game/CropCrazy/UI/BC_WBP_P1BuyShop.BT_BeetAmount` _returnvalue_3))
    (else
      (bind _returnvalue_4 (`|CreateWidget` "/Game/CropCrazy/UI/BC_WBP_P2BuyShop.BC_WBP_P2BuyShop_C" _returnvalue))
      (`UserWidget.AddToViewport` _returnvalue_4 0)
      (`WidgetBlueprintLibrary.SetInputMode_GameAndUIEx` _returnvalue null)
      (`Controller.SetIgnoreLookInput` _returnvalue true)
      ;[0 1 0] Add Controller Support to Player 2 Buy Shop
      (`Widget.SetKeyboardFocus` (`/Game/CropCrazy/UI/BC_WBP_P2BuyShop.BT_BeetAmount` _returnvalue_4)))))

(event `self.Interact.OnComponentEndOverlap`
  (params (OverlappedComponent :type "PrimitiveComponent Object Reference") (OtherActor :type "Actor Object Reference") (OtherComp :type "PrimitiveComponent Object Reference") (OtherBodyIndex :type Integer))
  (bind _returnvalue (`GameplayStatics.GetPlayerController` 0))
  ;[0 1 0] When Player 1 Moves Away From the Shop, Close the "Buy Shop" Widget
  (if (not (== OverlappedComponent _returnvalue))
    (`Widget.RemoveFromParent` (stale `self.Interact.OnComponentBeginOverlap` _returnvalue_3))
    (`Widget.RemoveFromParent` (stale `self.Interact.OnComponentBeginOverlap` _returnvalue_4))
    (`WidgetBlueprintLibrary.SetInputMode_GameOnly` _returnvalue)
    (set `PlayerController.bShowMouseCursor` false _returnvalue)
    (bind _returnvalue_2 (`|CreateWidget` "/Game/CropCrazy/UI/BC_WBP_HUD.BC_WBP_HUD_C"))
    (`UserWidget.AddToViewport` _returnvalue_2 0)))

(fn `UserConstructionScript`)
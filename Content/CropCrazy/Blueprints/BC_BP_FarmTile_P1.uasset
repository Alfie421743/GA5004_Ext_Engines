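; Player-one farm tile in CropCrazy that grows beetroot, mushroom or pumpkin from the player's selected seed, using up one seed.
; Each crop event swaps static meshes through growing, watering, harvest and decay stages, timed by a countdown macro shown on 3D text.
; Unwatered or unharvested crops decay, while harvesting spawns the matching pickup actor.
; Text is angled toward a camera actor at BeginPlay, and player overlap reveals a billboard.
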(event `self.ReceiveBeginPlay`
  ;[0 1 0] Set Text
  (set `Text3DComponent.Text` (`self.Value`) (`self.TXT_Time`))
  ;[0 1 0] Reference the Player
  (bind _asbc_bp_third_person_character (cast `/Game/CropCrazy/ThirdPerson/Blueprints/BC_BP_ThirdPersonCharacter` (`GameplayStatics.GetPlayerCharacter` 0)))
  (set `self.REF_Character` _asbc_bp_third_person_character)
  ;[0 1 0] Custom Event "E_RotateText"
  (`self.E_RotateText`))

(event `/Game/CropCrazy/Blueprints/BPIs/BC_BPI_PlantSeed.PlantSeed`
  ;[0 1 0] Plant Seed Based on Selected Item
  (if (not (`self.SomethingPlanted?`))
    (switch `int` (`/Game/CropCrazy/ThirdPerson/Blueprints/BC_BP_ThirdPersonCharacter.P1Seed` (`self.REF_Character`))
      (:`0`
        (`self.M_BeetrootSeed?`
          (:`Output`
            (`self.E_Plant_Beetroot`))))
      (:`1`
        (`self.M_MushroomSeed?`
          (:`Output`
            (`self.E_PlantMushroom`))))
      (:`2`
        (`self.M_PumpkinSeed?`
          (:`Output`
            (`self.E_PlantPumpkin`)))))
    (set `self.SomethingPlanted?` true)))

(event `E_Plant_Beetroot`
  (bind _relativetransformlocation (`self.RelativeTransformLocation`))
  ;[0 1 0] Plant Beetroot
  (bind _returnvalue (`AddComponent|NODE_AddStaticMeshComponent-0` :`RelativeTransform` (`KismetMathLibrary.MakeTransform` _relativetransformlocation)))
  (set `Text3DComponent.Text` "Growing" (`self.TXT_Stages`))
  (set `self.Growing?` true)
  (`self.M_Grow_Time` (`self.BeetrootGrowTime`)
    (:`Out`
      (`ActorComponent.K2_DestroyComponent` _returnvalue)
      (set `self.Growing?` false)
      (bind _returnvalue_2 (`AddComponent|NODE_AddStaticMeshComponent-1` :`RelativeTransform` (`KismetMathLibrary.MakeTransform` _relativetransformlocation)))
      (set `Text3DComponent.Text` "Water" (`self.TXT_Stages`))
      (`self.M_Grow_Time` (`KismetMathLibrary.RandomIntegerInRange` 5 8)
        (:`Out`
          (if (`self.Watered?`)
            (`ActorComponent.K2_DestroyComponent` _returnvalue_2)
            (bind _returnvalue_3 (`AddComponent|NODE_AddStaticMeshComponent-2` :`RelativeTransform` (`KismetMathLibrary.MakeTransform` _relativetransformlocation)))
            (set `Text3DComponent.Text` "Harvest" (`self.TXT_Stages`))
            (set `self.FullyGrown?` true)
            (set `self.CurrentMesh` _returnvalue_3)
            (set `self.WhatCanBeHarvested` "Beetroot")
            ;[0 1 0] Random Decay for Beetroots
            (`self.M_Grow_Time` (`KismetMathLibrary.RandomIntegerInRange` 4 7)
              (:`Out`
                (if (`self.FullyGrown?`)
                  (`ActorComponent.K2_DestroyComponent` _returnvalue_3 :!label _label)
                  (`ActorComponent.K2_DestroyComponent` _returnvalue_2)
                  (set `Text3DComponent.Text` "Decayed" (`self.TXT_Stages`))
                  (bind _returnvalue_4 (`AddComponent|NODE_AddStaticMeshComponent-10` :`RelativeTransform` (`KismetMathLibrary.MakeTransform` _relativetransformlocation)))
                  (set `self.WhatCanBeHarvested` "")
                  (set `self.Decayed` true)
                  (`KismetSystemLibrary.Delay` 5.0)
                  (`ActorComponent.K2_DestroyComponent` _returnvalue_4)
                  (set `self.SomethingPlanted?` false)
                  (set `Text3DComponent.Text` "" (`self.TXT_Stages`)))))
            (else
              (goto _label))))))))

(event `E_PlantMushroom`
  (bind _relativetransformlocation (`self.RelativeTransformLocation`))
  ;[0 1 0.001] Plant Mushroom
  (bind _returnvalue (`AddComponent|NODE_AddStaticMeshComponent-3` :`RelativeTransform` (`KismetMathLibrary.MakeTransform` _relativetransformlocation)))
  (set `Text3DComponent.Text` "Growing" (`self.TXT_Stages`))
  (set `self.Growing?` true)
  (`self.M_Grow_Time` (`self.MushroomGrowTime`)
    (:`Out`
      (`ActorComponent.K2_DestroyComponent` _returnvalue)
      (set `self.Growing?` false)
      (bind _returnvalue_2 (`AddComponent|NODE_AddStaticMeshComponent-4` :`RelativeTransform` (`KismetMathLibrary.MakeTransform` _relativetransformlocation)))
      (set `Text3DComponent.Text` "Water" (`self.TXT_Stages`))
      (`self.M_Grow_Time` (`KismetMathLibrary.RandomIntegerInRange` 5 8)
        (:`Out`
          (if (`self.Watered?`)
            (`ActorComponent.K2_DestroyComponent` _returnvalue_2)
            (bind _returnvalue_3 (`AddComponent|NODE_AddStaticMeshComponent-5` :`RelativeTransform` (`KismetMathLibrary.MakeTransform` _relativetransformlocation)))
            (set `Text3DComponent.Text` "Harvest" (`self.TXT_Stages`))
            (set `self.FullyGrown?` true)
            (set `self.CurrentMesh` _returnvalue_3)
            (set `self.WhatCanBeHarvested` "Mushroom")
            ;[0 1 0] Random Decay for Mushrooms
            (`self.M_Grow_Time` (`KismetMathLibrary.RandomIntegerInRange` 4 7)
              (:`Out`
                (if (`self.FullyGrown?`)
                  (`ActorComponent.K2_DestroyComponent` _returnvalue_3 :!label _label_2)
                  (`ActorComponent.K2_DestroyComponent` _returnvalue_2)
                  (set `Text3DComponent.Text` "Decayed" (`self.TXT_Stages`))
                  (bind _returnvalue_4 (`AddComponent|NODE_AddStaticMeshComponent-11` :`RelativeTransform` (`KismetMathLibrary.MakeTransform` _relativetransformlocation)))
                  (set `self.WhatCanBeHarvested` "")
                  (`KismetSystemLibrary.Delay` 5.0)
                  (`ActorComponent.K2_DestroyComponent` _returnvalue_4)
                  (set `self.SomethingPlanted?` false))))
            (else
              (goto _label_2))))))))

(event `E_PlantPumpkin`
  (bind _relativetransformlocation (`self.RelativeTransformLocation`))
  ;[0 1 0] Plant Pumpkin
  (bind _returnvalue (`AddComponent|NODE_AddStaticMeshComponent-6` :`RelativeTransform` (`KismetMathLibrary.MakeTransform` _relativetransformlocation)))
  (set `Text3DComponent.Text` "Growing" (`self.TXT_Stages`))
  (set `self.Growing?` true)
  (`self.M_Grow_Time` (`self.PumpkinGrowTime`)
    (:`Out`
      (`ActorComponent.K2_DestroyComponent` _returnvalue)
      (set `self.Growing?` false)
      (bind _returnvalue_2 (`AddComponent|NODE_AddStaticMeshComponent-7` :`RelativeTransform` (`KismetMathLibrary.MakeTransform` _relativetransformlocation)))
      (set `Text3DComponent.Text` "Water" (`self.TXT_Stages`))
      (`self.M_Grow_Time` (`KismetMathLibrary.RandomIntegerInRange` 5 8)
        (:`Out`
          (if (`self.Watered?`)
            (`ActorComponent.K2_DestroyComponent` _returnvalue_2)
            (bind _returnvalue_3 (`AddComponent|NODE_AddStaticMeshComponent-8` :`RelativeTransform` (`KismetMathLibrary.MakeTransform` _relativetransformlocation)))
            (set `Text3DComponent.Text` "Harvest" (`self.TXT_Stages`))
            (set `self.FullyGrown?` true)
            (set `self.CurrentMesh` _returnvalue_3)
            (set `self.WhatCanBeHarvested` "Pumpkin")
            ;[0 1 0] Random Decay for Pumpkins
            (`self.M_Grow_Time` (`KismetMathLibrary.RandomIntegerInRange` 4 7)
              (:`Out`
                (if (`self.FullyGrown?`)
                  (`ActorComponent.K2_DestroyComponent` _returnvalue_3 :!label _label_3)
                  (`ActorComponent.K2_DestroyComponent` _returnvalue_2)
                  (set `Text3DComponent.Text` "Decayed" (`self.TXT_Stages`))
                  (bind _returnvalue_4 (`AddComponent|NODE_AddStaticMeshComponent-14` :`RelativeTransform` (`KismetMathLibrary.MakeTransform` _relativetransformlocation)))
                  (set `self.WhatCanBeHarvested` "")
                  (`KismetSystemLibrary.Delay` 5.0)
                  (`ActorComponent.K2_DestroyComponent` _returnvalue_4)
                  (set `self.SomethingPlanted?` false))))
            (else
              (goto _label_3))))))))

(event `self.Interaction.OnComponentBeginOverlap`
  (params (OverlappedComponent :type "PrimitiveComponent Object Reference") (OtherActor :type "Actor Object Reference") (OtherComp :type "PrimitiveComponent Object Reference") (OtherBodyIndex :type Integer) (bFromSweep :type Boolean) (SweepResult :type "HitResult Structure (by ref)"))
  ;[0 1 0] Add UI to Crop Plot
  (if (== OtherActor (`self.REF_Character`))
    (`SceneComponent.SetVisibility` (`self.Billboard`) true false)))

(event `E_RotateText`
  ;[0 1 0] Rotate Text to Face Player
  (bind _returnvalue (`GameplayStatics.GetActorOfClass` "/Game/CropCrazy/Blueprints/BC_BP_CameraMoved.BC_BP_CameraMoved_C"))
  (bind (_returnvalue_roll _returnvalue_pitch _returnvalue_yaw) (`KismetMathLibrary.BreakRotator` (`KismetMathLibrary.FindLookAtRotation` (`SceneComponent.K2_GetComponentLocation` (`self.TXT_Time`)) (`SceneComponent.K2_GetComponentLocation` (`Actor.RootComponent` _returnvalue)))))
  (`SceneComponent.K2_SetWorldRotation` (`self.TXT_Time`) (`KismetMathLibrary.MakeRotator` _returnvalue_roll (- _returnvalue_pitch 60.0) (- _returnvalue_yaw 180.0)) false false)
  (bind (_returnvalue_roll_2 _returnvalue_pitch_2 _returnvalue_yaw_2) (`KismetMathLibrary.BreakRotator` (`KismetMathLibrary.FindLookAtRotation` (`SceneComponent.K2_GetComponentLocation` (`self.TXT_Stages`)) (`SceneComponent.K2_GetComponentLocation` (`Actor.RootComponent` _returnvalue)))))
  (`SceneComponent.K2_SetWorldRotation` (`self.TXT_Stages`) (`KismetMathLibrary.MakeRotator` _returnvalue_roll_2 (- _returnvalue_pitch_2 60.0) (- _returnvalue_yaw_2 180.0)) false false))

(event `self.Interaction.OnComponentEndOverlap`
  (params (OverlappedComponent :type "PrimitiveComponent Object Reference") (OtherActor :type "Actor Object Reference") (OtherComp :type "PrimitiveComponent Object Reference") (OtherBodyIndex :type Integer))
  ;[0 1 0] Add UI to Crop Plot
  (if (not (== OverlappedComponent (`self.REF_Character`)))
    (`SceneComponent.SetVisibility` (`self.Billboard`) false false)))

(event `/Game/CropCrazy/Blueprints/BPIs/BC_BPI_Activate.Activate`
  ;[0 1 0] Harvest Plant
  (`self.F_Harvest`))

(fn `F_Harvest`
  (bind _returnvalue (`KismetMathLibrary.Conv_VectorToTransform` (`SceneComponent.K2_GetComponentLocation` (`self.TXT_Time`))))
  ;[0 1 0] Harvest Fully Grown Crops
  (if (`self.FullyGrown?`)
    (`ActorComponent.K2_DestroyComponent` (`self.CurrentMesh`))
    (switch `string` (`self.WhatCanBeHarvested`)
      (:`Default`
        _)
      (:`Beetroot`
        (`|SpawnActorFromClass` "/Game/CropCrazy/Blueprints/CropHarvest/BC_BP_BeetrootHarvested.BC_BP_BeetrootHarvested_C" _returnvalue "Undefined" "MultiplyWithRoot" null null))
      (:`Mushroom`
        (`|SpawnActorFromClass` "/Game/CropCrazy/Blueprints/CropHarvest/BC_BP_MushroomHarvested.BC_BP_MushroomHarvested_C" _returnvalue "Undefined" "MultiplyWithRoot" null null))
      (:`Pumpkin`
        (`|SpawnActorFromClass` "/Game/CropCrazy/Blueprints/CropHarvest/BC_BP_PumpkinHarvested.BC_BP_PumpkinHarvested_C" _returnvalue "Undefined" "MultiplyWithRoot" null null)))
    (set `self.FullyGrown?` false)
    (set `self.CurrentMesh` null)
    (set `self.SomethingPlanted?` false)
    (set `self.WhatCanBeHarvested` "")
    (set `Text3DComponent.Text` "" (`self.TXT_Stages`))))

(fn `UserConstructionScript`)
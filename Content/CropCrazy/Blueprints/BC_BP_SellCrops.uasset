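; Crop-selling trigger for CropCrazy that turns the player's harvested crops into score.
; Caches the player character on BeginPlay, then runs a sell function for beetroot, mushroom and pumpkin when that character overlaps the Box.
; Each function zeroes the crop count and adds a fixed per-unit score, with mushrooms worth more than beetroot and pumpkins most.
; Hardcoded branch chains handle only one to five units, so larger stacks are left unsold.
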(event `self.ReceiveBeginPlay`
  ;[0 1 0] Reference the player
  (bind _asbc_bp_third_person_character (cast `/Game/CropCrazy/ThirdPerson/Blueprints/BC_BP_ThirdPersonCharacter` (`GameplayStatics.GetPlayerCharacter` 0)))
  (set `self.REF_Character` _asbc_bp_third_person_character))

(event `self.Box.OnComponentBeginOverlap`
  (params (OverlappedComponent :type "PrimitiveComponent Object Reference") (OtherActor :type "Actor Object Reference") (OtherComp :type "PrimitiveComponent Object Reference") (OtherBodyIndex :type Integer) (bFromSweep :type Boolean) (SweepResult :type "HitResult Structure (by ref)"))
  (if (== OtherActor (`self.REF_Character`))
    (`self.F_SellBeetroot`)
    (`self.F_SellMushroom`)
    (`self.F_SellPumpkin`)))

(fn `F_SellBeetroot`
  (bind _ref_character (`self.REF_Character`))
  (bind _beetrootamount (`/Game/CropCrazy/ThirdPerson/Blueprints/BC_BP_ThirdPersonCharacter.BeetrootAmount` _ref_character))
  (bind _score (`/Game/CropCrazy/ThirdPerson/Blueprints/BC_BP_ThirdPersonCharacter.Score` _ref_character))
  (if (== _beetrootamount 1)
    (set `/Game/CropCrazy/ThirdPerson/Blueprints/BC_BP_ThirdPersonCharacter.BeetrootAmount` (- _beetrootamount 1) _ref_character)
    (set `/Game/CropCrazy/ThirdPerson/Blueprints/BC_BP_ThirdPersonCharacter.Score` (+ _score 3) _ref_character)
    (return)
    (elif (== _beetrootamount 2)
      (set `/Game/CropCrazy/ThirdPerson/Blueprints/BC_BP_ThirdPersonCharacter.BeetrootAmount` (- _beetrootamount 2) _ref_character)
      (set `/Game/CropCrazy/ThirdPerson/Blueprints/BC_BP_ThirdPersonCharacter.Score` (+ _score 6) _ref_character)
      (return)
      (elif (== _beetrootamount 3)
        (set `/Game/CropCrazy/ThirdPerson/Blueprints/BC_BP_ThirdPersonCharacter.BeetrootAmount` (- _beetrootamount 3) _ref_character)
        (set `/Game/CropCrazy/ThirdPerson/Blueprints/BC_BP_ThirdPersonCharacter.Score` (+ _score 9) _ref_character)
        (return)
        (elif (== _beetrootamount 4)
          (set `/Game/CropCrazy/ThirdPerson/Blueprints/BC_BP_ThirdPersonCharacter.BeetrootAmount` (- _beetrootamount 4) _ref_character)
          (set `/Game/CropCrazy/ThirdPerson/Blueprints/BC_BP_ThirdPersonCharacter.Score` (+ _score 12) _ref_character)
          (return)
          (elif (== _beetrootamount 5)
            (set `/Game/CropCrazy/ThirdPerson/Blueprints/BC_BP_ThirdPersonCharacter.BeetrootAmount` (- _beetrootamount 5) _ref_character)
            (set `/Game/CropCrazy/ThirdPerson/Blueprints/BC_BP_ThirdPersonCharacter.Score` (+ _score 15) _ref_character)
            (return)))))))

(fn `F_SellMushroom`
  (bind _ref_character (`self.REF_Character`))
  (bind _mushroomamount (`/Game/CropCrazy/ThirdPerson/Blueprints/BC_BP_ThirdPersonCharacter.MushroomAmount` _ref_character))
  (bind _score (`/Game/CropCrazy/ThirdPerson/Blueprints/BC_BP_ThirdPersonCharacter.Score` _ref_character))
  (if (== _mushroomamount 1)
    (set `/Game/CropCrazy/ThirdPerson/Blueprints/BC_BP_ThirdPersonCharacter.MushroomAmount` (- _mushroomamount 1) _ref_character)
    (set `/Game/CropCrazy/ThirdPerson/Blueprints/BC_BP_ThirdPersonCharacter.Score` (+ _score 5) _ref_character)
    (return)
    (elif (== _mushroomamount 2)
      (set `/Game/CropCrazy/ThirdPerson/Blueprints/BC_BP_ThirdPersonCharacter.MushroomAmount` (- _mushroomamount 2) _ref_character)
      (set `/Game/CropCrazy/ThirdPerson/Blueprints/BC_BP_ThirdPersonCharacter.Score` (+ _score 10) _ref_character)
      (return)
      (elif (== _mushroomamount 3)
        (set `/Game/CropCrazy/ThirdPerson/Blueprints/BC_BP_ThirdPersonCharacter.MushroomAmount` (- _mushroomamount 3) _ref_character)
        (set `/Game/CropCrazy/ThirdPerson/Blueprints/BC_BP_ThirdPersonCharacter.Score` (+ _score 15) _ref_character)
        (return)
        (elif (== _mushroomamount 4)
          (set `/Game/CropCrazy/ThirdPerson/Blueprints/BC_BP_ThirdPersonCharacter.MushroomAmount` (- _mushroomamount 4) _ref_character)
          (set `/Game/CropCrazy/ThirdPerson/Blueprints/BC_BP_ThirdPersonCharacter.Score` (+ _score 20) _ref_character)
          (return)
          (elif (== _mushroomamount 5)
            (set `/Game/CropCrazy/ThirdPerson/Blueprints/BC_BP_ThirdPersonCharacter.MushroomAmount` (- _mushroomamount 5) _ref_character)
            (set `/Game/CropCrazy/ThirdPerson/Blueprints/BC_BP_ThirdPersonCharacter.Score` (+ _score 25) _ref_character)
            (return)))))))

(fn `F_SellPumpkin`
  (bind _ref_character (`self.REF_Character`))
  (bind _pumpkinamount (`/Game/CropCrazy/ThirdPerson/Blueprints/BC_BP_ThirdPersonCharacter.PumpkinAmount` _ref_character))
  (bind _score (`/Game/CropCrazy/ThirdPerson/Blueprints/BC_BP_ThirdPersonCharacter.Score` _ref_character))
  (if (== _pumpkinamount 1)
    (set `/Game/CropCrazy/ThirdPerson/Blueprints/BC_BP_ThirdPersonCharacter.PumpkinAmount` (- _pumpkinamount 1) _ref_character)
    (set `/Game/CropCrazy/ThirdPerson/Blueprints/BC_BP_ThirdPersonCharacter.Score` (+ _score 8) _ref_character)
    (return)
    (elif (== _pumpkinamount 2)
      (set `/Game/CropCrazy/ThirdPerson/Blueprints/BC_BP_ThirdPersonCharacter.PumpkinAmount` (- _pumpkinamount 2) _ref_character)
      (set `/Game/CropCrazy/ThirdPerson/Blueprints/BC_BP_ThirdPersonCharacter.Score` (+ _score 16) _ref_character)
      (return)
      (elif (== _pumpkinamount 3)
        (set `/Game/CropCrazy/ThirdPerson/Blueprints/BC_BP_ThirdPersonCharacter.PumpkinAmount` (- _pumpkinamount 3) _ref_character)
        (set `/Game/CropCrazy/ThirdPerson/Blueprints/BC_BP_ThirdPersonCharacter.Score` (+ _score 24) _ref_character)
        (return)
        (elif (== _pumpkinamount 4)
          (set `/Game/CropCrazy/ThirdPerson/Blueprints/BC_BP_ThirdPersonCharacter.PumpkinAmount` (- _pumpkinamount 4) _ref_character)
          (set `/Game/CropCrazy/ThirdPerson/Blueprints/BC_BP_ThirdPersonCharacter.Score` (+ _score 32) _ref_character)
          (return)
          (elif (== _pumpkinamount 5)
            (set `/Game/CropCrazy/ThirdPerson/Blueprints/BC_BP_ThirdPersonCharacter.PumpkinAmount` (- _pumpkinamount 5) _ref_character)
            (set `/Game/CropCrazy/ThirdPerson/Blueprints/BC_BP_ThirdPersonCharacter.Score` (+ _score 40) _ref_character)
            (return)))))))

(fn `UserConstructionScript`)
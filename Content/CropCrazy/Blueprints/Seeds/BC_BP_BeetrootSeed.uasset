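; Beetroot seed pickup that adds to the player's beetroot seed count when touched.
; On BeginPlay it casts player character 0 to BC_BP_ThirdPersonCharacter and caches the reference.
; When that character begins overlapping the Box component, it increments BeetrootSeeds on the character and destroys itself.
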(event `self.ReceiveBeginPlay`
  ;[0 1 0] Cast to Player
  (bind _asbc_bp_third_person_character (cast `/Game/CropCrazy/ThirdPerson/Blueprints/BC_BP_ThirdPersonCharacter` (`GameplayStatics.GetPlayerCharacter` 0)))
  (set `self.REF_Character` _asbc_bp_third_person_character))

(event `self.Box.OnComponentBeginOverlap`
  (params (OverlappedComponent :type "PrimitiveComponent Object Reference") (OtherActor :type "Actor Object Reference") (OtherComp :type "PrimitiveComponent Object Reference") (OtherBodyIndex :type Integer) (bFromSweep :type Boolean) (SweepResult :type "HitResult Structure (by ref)"))
  (bind _ref_character (`self.REF_Character`))
  ;[0 1 0] Give the player a beetroot seed and destroy the mesh
  (if (== OtherActor _ref_character)
    (set `/Game/CropCrazy/ThirdPerson/Blueprints/BC_BP_ThirdPersonCharacter.BeetrootSeeds` (+ (`/Game/CropCrazy/ThirdPerson/Blueprints/BC_BP_ThirdPersonCharacter.BeetrootSeeds` _ref_character) 1) _ref_character)
    (`self.K2_DestroyActor`)))

(fn `UserConstructionScript`)
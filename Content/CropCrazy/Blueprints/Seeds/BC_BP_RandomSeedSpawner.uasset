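; Crop Crazy spawner actor that continuously spawns beetroot, mushroom and pumpkin seeds at its root location.
; On BeginPlay it casts and stores the player character, starting the timers only if that cast succeeds.
; Each seed type has its own looping timer, with a random interval rolled once at start rather than on each spawn.
; Only the beetroot spawn explicitly overrides collision handling to always spawn.
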(event `self.ReceiveBeginPlay`
  (bind _returnvalue (`KismetMathLibrary.RandomFloatInRange` 2.0 4.0))
  ;[0 1 0] Cast to player
  (bind _asbc_bp_third_person_character (cast `/Game/CropCrazy/ThirdPerson/Blueprints/BC_BP_ThirdPersonCharacter` (`GameplayStatics.GetPlayerCharacter` 0)))
  (set `self.REF_Character` _asbc_bp_third_person_character)
  ;[0 1 0] Spawn Beetroot Seed
  (`KismetSystemLibrary.K2_SetTimerDelegate` (delegate `E_SpawnBeetSeeds`) _returnvalue true)
  ;[0 1 0] Spawn Mushroom Seed
  (`KismetSystemLibrary.K2_SetTimerDelegate` (delegate `E_SpawnMushroomSeed`) _returnvalue true)
  ;[0 1 0] Spawn Pumpkin Seed
  (`KismetSystemLibrary.K2_SetTimerDelegate` (delegate `E_SpawnPumpkinSeeds`) _returnvalue true))

(event `E_SpawnBeetSeeds`
  ;[0 1 0] Spawn Beetroot Seed
  (`|SpawnActorFromClass` "/Game/CropCrazy/Blueprints/Seeds/BC_BP_BeetrootSeed.BC_BP_BeetrootSeed_C" (`KismetMathLibrary.Conv_VectorToTransform` (`SceneComponent.K2_GetComponentLocation` (`self.DefaultSceneRoot`))) "AlwaysSpawn" "MultiplyWithRoot" null null))

(event `E_SpawnMushroomSeed`
  ;[0 1 0] Spawn Mushroom Seed
  (`|SpawnActorFromClass` "/Game/CropCrazy/Blueprints/Seeds/BC_BP_MushroomSeed.BC_BP_MushroomSeed_C" (`KismetMathLibrary.Conv_VectorToTransform` (`SceneComponent.K2_GetComponentLocation` (`self.DefaultSceneRoot`))) "Undefined" "MultiplyWithRoot" null null))

(event `E_SpawnPumpkinSeeds`
  ;[0 1 0] Spawn Pumpkin Seed
  (`|SpawnActorFromClass` "/Game/CropCrazy/Blueprints/Seeds/BC_BP_PumpkinSeed.BC_BP_PumpkinSeed_C" (`KismetMathLibrary.Conv_VectorToTransform` (`SceneComponent.K2_GetComponentLocation` (`self.DefaultSceneRoot`))) "Undefined" "MultiplyWithRoot" null null))

(fn `UserConstructionScript`)
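; Sumo game arena that shrinks over time and penalises characters who leave its bounds.
; A looping 20-second timer reduces the Cylinder's X and Y scale by a fixed step, with no minimum clamp.
; When an AP_BP_SumoCharacter stops overlapping the Sphere, it is teleported to a random elevated point around the world origin and loses a life.
; The Box overlap event is empty.
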(event `self.ReceiveBeginPlay`
  (`KismetSystemLibrary.K2_SetTimerDelegate` (delegate `E_Shrink`) 20.0 true))

(event `E_Shrink`
  (bind _cylinder (`self.Cylinder`))
  (bind (_returnvalue_x _returnvalue_y _returnvalue_z) (`KismetMathLibrary.BreakVector` (`SceneComponent.K2_GetComponentScale` _cylinder)))
  (`SceneComponent.SetWorldScale3D` _cylinder (`KismetMathLibrary.MakeVector` (- _returnvalue_x 0.75) (- _returnvalue_y 0.75) _returnvalue_z)))

(event `self.Box.OnComponentBeginOverlap`
  (params (OverlappedComponent :type "PrimitiveComponent Object Reference") (OtherActor :type "Actor Object Reference") (OtherComp :type "PrimitiveComponent Object Reference") (OtherBodyIndex :type Integer) (bFromSweep :type Boolean) (SweepResult :type "HitResult Structure (by ref)")))

(event `self.Sphere.OnComponentEndOverlap`
  (params (OverlappedComponent :type "PrimitiveComponent Object Reference") (OtherActor :type "Actor Object Reference") (OtherComp :type "PrimitiveComponent Object Reference") (OtherBodyIndex :type Integer))
  (bind _asap_bp_sumo_character (cast `/Game/SumoGame/Blueprint/Character/AP_BP_SumoCharacter` OtherActor))
  (`|ExecutionSequence`
    (:`then_0`
      (`self.K2_TeleportTo` :`self` _asap_bp_sumo_character :`DestLocation` (`KismetMathLibrary.MakeVector` (`KismetMathLibrary.RandomFloatInRange` -400.0 400.0) (`KismetMathLibrary.RandomFloatInRange` -400.0 400.0) 400.0)))
    (:`then_1`
      (`/Game/SumoGame/Blueprint/Character/AP_BP_SumoCharacter.E_LoseLife` _asap_bp_sumo_character))))

(fn `UserConstructionScript`)
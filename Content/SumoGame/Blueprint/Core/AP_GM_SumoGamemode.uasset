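; Game mode for a two-player local sumo game that runs the match countdown and the menus around it.
; BeginPlay creates a second local player, shows the main menu with Start focused, caches both player characters and starts the countdown immediately.
; A looping one-second timer decrements Timer and shows a "Time's up" end menu at zero; it is never cleared here, so that menu is recreated every second afterwards.
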(event `self.ReceiveBeginPlay`
  (`GameplayStatics.CreatePlayer` 1)
  (bind _returnvalue (`|CreateWidget` "/Game/SumoGame/UMG/AP_WBP_MainMenu.AP_WBP_MainMenu_C"))
  (`UserWidget.AddToViewport` _returnvalue 0)
  (`self.E_SetUpTimer`)
  (bind _asap_bpc_player_1 (cast `/Game/SumoGame/Blueprint/Character/AP_BPC_Player1` (`GameplayStatics.GetPlayerCharacter` 0)))
  (set `self.Ref_Player1` _asap_bpc_player_1)
  (bind _asap_bpc_player_2 (cast `/Game/SumoGame/Blueprint/Character/AP_BPC_Player2` (`GameplayStatics.GetPlayerCharacter` 1)))
  (set `self.Ref_Player2` _asap_bpc_player_2)
  (`Widget.SetKeyboardFocus` (`/Game/SumoGame/UMG/AP_WBP_MainMenu.Btn_Start` _returnvalue)))

(event `E_SetUpTimer`
  (`KismetSystemLibrary.K2_SetTimerDelegate` (delegate `E_Timer`) 1.0 true))

(event `E_Timer`
  (`/Engine/EditorBlueprintResources/StandardMacros.DecrementInt` (`self.Timer`)
    (:`  `
      (if (<= (`self.Timer`) 0)
        (bind _returnvalue (`|CreateWidget` "/Game/SumoGame/UMG/AP_WBP_EndMenu.AP_WBP_EndMenu_C"))
        (set `TextBlock.Text` "Time's up" (`/Game/SumoGame/UMG/AP_WBP_EndMenu.Txt_Title` _returnvalue))
        (`UserWidget.AddToViewport` _returnvalue 0)
        (`Widget.SetKeyboardFocus` (`/Game/SumoGame/UMG/AP_WBP_EndMenu.Btn_Exit` _returnvalue))))))

(fn `UserConstructionScript`)
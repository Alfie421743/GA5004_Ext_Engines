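; Bowling pin spawner actor that builds, respawns and refills a triangular rack of physics-simulated cube mesh pins.
; Respawning clears current pins and derives the row count from MaxPins, then chained looping timers add pins row by row relative to an anchor component.
; Hit pins are destroyed and their stored positions moved to MissingPins, which the fill event replays on a timer without ever clearing the list.
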(event `ce_respawnPins`
  (bind (_returnvalue_x _returnvalue_y _returnvalue_z) (`KismetMathLibrary.BreakVector` (`self.K2_GetActorLocation`)))
  (bind _timerpinspawner01 (`self.timerPinSpawner01`))
  (set `self.Index` 0)
  (set `self.pinCalcs01` 0)
  (set `self.pinCalcs02` 0)
  (set `self.pinCalcs03` 0)
  (set `self.timerPinSpawner01` 0)
  (set `self.timerPinSpawner02` 0)
  (for _array_element (`self.currentPins`)
    (`ActorComponent.K2_DestroyComponent` _array_element))
  (`KismetArrayLibrary.Array_Clear` (`self.currentPins`))
  (for _ (range 1 (+ (`self.maxPins`) 1)) :!label _label
    (bind _result (`/Engine/EditorBlueprintResources/StandardMacros.IncrementInt` (`self.pinCalcs01`))
      (:`  `
        (bind _output_get (set `self.pinCalcs02` (+ _result (`self.pinCalcs02`))))
        (if (>= _output_get (`self.maxPins`))
          (break)))))
  (bind _returnvalue (`AddComponent|NODE_AddStaticMeshComponent-1` :`RelativeTransform` (`KismetMathLibrary.MakeTransform` (`KismetMathLibrary.MakeVector` (+ (- _returnvalue_x 5000.0) (* (`self.maxPins`) 16.0)) (+ _returnvalue_y (+ (* (`self.pinCalcs01`) 64.0) 64)) _returnvalue_z) (struct) (0.3 0.3 1.0))))
  (bind _output_get_2 (set `self.firstPin` _returnvalue))
  (`KismetSystemLibrary.Delay` 0.4)
  (if (not (>= _timerpinspawner01 (`self.pinCalcs01`))) :!label _label_2
    (`/Engine/EditorBlueprintResources/StandardMacros.IncrementInt` _timerpinspawner01
      (:`  `
        (bind _returnvalue_2 (`KismetSystemLibrary.K2_SetTimerDelegate` (delegate `ce_timerPinSpawner01`) 0.17 true))))))

(event `ce_fillPins`
  (bind _returnvalue (`KismetSystemLibrary.K2_SetTimerDelegate` (delegate `ce_timerPinSpawner02`) 0.17 true)))

(event `ce_timerPinSpawner02`
  (bind _missingpins (`self.missingPins`))
  (bind _relative_transform_location_x (`self.Relative Transform Location X`))
  (bind _relative_transform_location_y (`self.Relative Transform Location Y`))
  (bind _relative_transform_location_z (`self.Relative Transform Location Z`))
  (bind _timerpinspawner03 (`self.timerPinSpawner03`))
  (bind (_output_x _output_y _output_z) (`KismetMathLibrary.BreakVector` (`|GetArrayItem` _missingpins (`self.timerPinSpawner03`))))
  (bind _returnvalue (- _relative_transform_location_z 900.0))
  (if (>= _timerpinspawner03 (`KismetArrayLibrary.Array_Length` _missingpins))
    (`KismetSystemLibrary.K2_ClearAndInvalidateTimerHandle` (stale `ce_fillPins` _returnvalue))
    (set `self.timerPinSpawner03` 0)
    (else
      (set `self.Relative Transform Location X` _output_x)
      (set `self.Relative Transform Location Y` _output_y)
      (set `self.Relative Transform Location Z` _output_z)
      (`/Engine/EditorBlueprintResources/StandardMacros.IncrementInt` _timerpinspawner03
        (:`  `
          (bind _returnvalue_2 (`AddComponent|NODE_AddStaticMeshComponent-2` :`RelativeTransform` (`KismetMathLibrary.MakeTransform` (`KismetMathLibrary.MakeVector` (`self.Relative Transform Location X`) (`self.Relative Transform Location Y`) (`self.Relative Transform Location Z`)) (struct) (0.3 0.3 1.0)) :!label _label_3))
          (`StaticMeshComponent.SetStaticMesh` _returnvalue_2 "/Game/LollyPops/LevelPrototyping/Meshes/SM_ChamferCube.SM_ChamferCube")
          (`KismetSystemLibrary.MoveComponentTo` _returnvalue_2 (`KismetMathLibrary.MakeVector` _relative_transform_location_x _relative_transform_location_y _returnvalue) (struct) false true 0.1)
          (`KismetSystemLibrary.MoveComponentTo` _returnvalue_2 (`KismetMathLibrary.MakeVector` _relative_transform_location_x _relative_transform_location_y _returnvalue) (struct) false false 0.05)
          (`PrimitiveComponent.SetSimulatePhysics` _returnvalue_2 true)
          (bind _returnvalue_3 (`KismetArrayLibrary.Array_Add` (`self.currentPins`) _returnvalue_2))
          (`KismetArrayLibrary.Array_Set` (`self.currentPinsPos`) _returnvalue_3 (`KismetMathLibrary.MakeVector` _relative_transform_location_x _relative_transform_location_y _relative_transform_location_z) true)
          (`/Engine/EditorBlueprintResources/StandardMacros.IncrementInt` (`self.Index`)
            (:`  `
              (`KismetSystemLibrary.PrintString` (`KismetStringLibrary.Conv_IntToString` (`KismetArrayLibrary.Array_Length` (`self.currentPins`))) true true (struct :`G` 0.66 :`B` 1.0 :`A` 1.0) 20.0))))))))

(event `self.ReceiveBeginPlay`
  (goto _label))

(event `ce_spawnPins`
  (goto _label_2))

(event `ce_timerPinSpawner01`
  (bind _pincalcs03 (`self.pinCalcs03`))
  (bind _timerpinspawner02 (`self.timerPinSpawner02`))
  (bind _returnvalue (`SceneComponent.GetRelativeTransform` (`self.firstPin`)))
  (bind _returnvalue_2 (- (.y (.location _returnvalue)) (* (`self.timerPinSpawner02`) 128.0)))
  (if (>= _timerpinspawner02 (`self.pinCalcs01`))
    (`KismetSystemLibrary.K2_ClearAndInvalidateTimerHandle` (stale `ce_respawnPins` _returnvalue_2))
    (`/Engine/EditorBlueprintResources/StandardMacros.IncrementInt` _pincalcs03
      (:`  `
        (set `self.timerPinSpawner02` (`self.pinCalcs03`))
        (`self.ce_spawnPins`)))
    (else
      (`/Engine/EditorBlueprintResources/StandardMacros.IncrementInt` _timerpinspawner02
        (:`  `
          (if (>= _pincalcs03 1)
            (set `self.Relative Transform Location Y` (+ (* (`self.pinCalcs03`) 64) _returnvalue_2))
            (else
              (set `self.Relative Transform Location Y` _returnvalue_2)))
          (set `self.Relative Transform Location X` (- (.x (.location _returnvalue)) (* (`self.pinCalcs03`) 128.0)))
          (goto _label_3))))))

(event `self.ReceiveHit`
  (params (MyComp :type "PrimitiveComponent Object Reference") (Other :type "Actor Object Reference") (OtherComp :type "PrimitiveComponent Object Reference") (bSelfMoved :type Boolean) (HitLocation :type "Vector Structure") (HitNormal :type "Vector Structure") (NormalImpulse :type "Vector Structure") (Hit :type "HitResult Structure (by ref)"))
  (bind _currentpinspos (`self.currentPinsPos`))
  (bind _currentpins (`self.currentPins`))
  (for (_array_element _array_index) _currentpins
    (if (== _array_element MyComp)
      (`KismetArrayLibrary.Array_Add` (`self.missingPins`) (`|GetArrayItem` _currentpinspos _array_index))
      (`ActorComponent.K2_DestroyComponent` _array_element)
      (`KismetArrayLibrary.Array_Remove` _currentpins _array_index)
      (`KismetArrayLibrary.Array_Remove` _currentpinspos _array_index)
      (for _array_element_2 (`self.missingPins`)
        (`KismetSystemLibrary.PrintString` (`KismetStringLibrary.Conv_VectorToString` _array_element_2) true true (struct :`G` 0.082511 :`B` 1.0 :`A` 1.0) 15.0)))))

(fn `UserConstructionScript`)
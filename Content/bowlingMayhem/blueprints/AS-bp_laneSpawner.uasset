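; Lane spawner actor that builds the bowling lane at runtime, segment by segment, and finishes it with a pin spawner.
; A looping timer started on BeginPlay increments a counter and spawns a lane actor at evenly spaced steps along world X.
; When the counter reaches its limit, the timer is cleared and the pin spawner is placed at the next step.
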(event `self.ReceiveBeginPlay`
  (bind _returnvalue (`KismetSystemLibrary.K2_SetTimerDelegate` (delegate `ce_laneTimer`) 0.15 true)))

(event `ce_laneTimer`
  (bind _result (`/Engine/EditorBlueprintResources/StandardMacros.IncrementInt` (`self.laneTimer`))
    (:`  `
      (if (< _result 9)
        (bind _returnvalue (`KismetMathLibrary.Conv_IntToDouble` (* _result 500)))
        (`|SpawnActorFromClass` "/Game/bowlingMayhem/blueprints/AS-bp_lane.AS-bp_lane_C" (`KismetMathLibrary.MakeTransform` (`KismetMathLibrary.MakeVector` _returnvalue)) "Undefined" "MultiplyWithRoot" null null)
        (else
          (`KismetSystemLibrary.K2_ClearAndInvalidateTimerHandle` (stale `self.ReceiveBeginPlay` _returnvalue))
          (`|SpawnActorFromClass` "/Game/bowlingMayhem/blueprints/AS-bp_pinSpawner.AS-bp_pinSpawner_C" (`KismetMathLibrary.MakeTransform` (`KismetMathLibrary.MakeVector` _returnvalue)) "Undefined" "MultiplyWithRoot" null null))))))

(fn `UserConstructionScript`)
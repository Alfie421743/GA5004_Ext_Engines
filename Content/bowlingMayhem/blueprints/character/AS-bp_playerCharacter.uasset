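; Player character Blueprint that handles basic look, move and jump controls through Enhanced Input actions.
; Look input drives controller yaw and pitch, while separate forward and right actions add movement input along directions derived only from control yaw, keeping movement level with the ground.
; The jump action calls the Character's built-in Jump, and the construction script is empty.
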(event `EnhancedInput|/Game/bowlingMayhem/inputs/AS-ia_look`
  (params (ActionValue :type "Vector2D Structure") (ElapsedSeconds :type "Float (double-precision)") (TriggeredSeconds :type "Float (double-precision)") (InputAction :type "InputAction Object Reference" :default "/Game/bowlingMayhem/inputs/AS-ia_look.AS-ia_look"))
  (:`Triggered`
    (`self.AddControllerYawInput` ActionValue_X)
    (`self.AddControllerPitchInput` ActionValue_Y)))

(event `EnhancedInput|/Game/bowlingMayhem/inputs/AS-ia_moveForward`
  (params (ActionValue :type "Float (double-precision)") (ElapsedSeconds :type "Float (double-precision)") (TriggeredSeconds :type "Float (double-precision)") (InputAction :type "InputAction Object Reference" :default "/Game/bowlingMayhem/inputs/AS-ia_moveForward.AS-ia_moveForward"))
  (bind (_returnvalue_roll _returnvalue_pitch _returnvalue_yaw) (`KismetMathLibrary.BreakRotator` (`self.GetControlRotation`)))
  (:`Triggered`
    (`self.AddMovementInput` (`KismetMathLibrary.GetForwardVector` (`KismetMathLibrary.MakeRotator` 0.0 0.0 _returnvalue_yaw)) ActionValue)))

(event `EnhancedInput|/Game/bowlingMayhem/inputs/AS-ia_moveRight`
  (params (ActionValue :type "Float (double-precision)") (ElapsedSeconds :type "Float (double-precision)") (TriggeredSeconds :type "Float (double-precision)") (InputAction :type "InputAction Object Reference" :default "/Game/bowlingMayhem/inputs/AS-ia_moveRight.AS-ia_moveRight"))
  (bind (_returnvalue_roll _returnvalue_pitch _returnvalue_yaw) (`KismetMathLibrary.BreakRotator` (`self.GetControlRotation`)))
  (:`Triggered`
    (`self.AddMovementInput` (`KismetMathLibrary.GetRightVector` (`KismetMathLibrary.MakeRotator` 0.0 0.0 _returnvalue_yaw)) ActionValue)))

(event `EnhancedInput|/Game/bowlingMayhem/inputs/AS-ia_jump`
  (params (ActionValue :type "Float (double-precision)") (ElapsedSeconds :type "Float (double-precision)") (TriggeredSeconds :type "Float (double-precision)") (InputAction :type "InputAction Object Reference" :default "/Game/bowlingMayhem/inputs/AS-ia_jump.AS-ia_jump"))
  (:`Triggered`
    (`self.Jump`)))

(fn `UserConstructionScript`)
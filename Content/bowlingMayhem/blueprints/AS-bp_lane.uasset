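; Bowling lane actor that animates its base mesh downward as play begins.
; On BeginPlay it makes the lane base visible, then uses MoveComponentTo to lower it along relative Z with an ease-out over one second.
; Disconnected copies of the same show-and-lower step, with shorter durations and no component assigned, remain in the graph and never run.
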(event `self.ReceiveBeginPlay`
  (bind _sm_lanebase (`self.sm_laneBase`))
  (bind _returnvalue (`SceneComponent.GetRelativeTransform` _sm_lanebase))
  (`SceneComponent.SetVisibility` _sm_lanebase true false)
  (`KismetSystemLibrary.MoveComponentTo` _sm_lanebase (`KismetMathLibrary.MakeVector` (.x (.location _returnvalue)) (.y (.location _returnvalue)) (- (.z (.location _returnvalue)) 1000.0)) (struct) true false 1.0))

(fn `UserConstructionScript`)